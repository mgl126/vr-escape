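; BP_BigButton is an escape room button that gives glowing visual feedback for being lit, winning or losing.
; The construction script creates a dynamic instance of M_Color on TriggerButton and tints it with the Color variable.
; Events drive that material's color and intensity: LightBigButton flashes briefly, while PlayBigVictory stays bright green.
; PlayBigError flashes red, then after a delay turns the glow off and restores the original color.
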(event `PlayBigVictory`
  ; Ganaste
  (`MaterialInstanceDynamic.SetVectorParameterValue` (`self.DynMat`) "Color" (struct :`G` 1.0 :`B` 0.178619 :`A` 1.0))
  (`MaterialInstanceDynamic.SetScalarParameterValue` (`self.DynMat`) "Intensity" 5.0))

(event `LightBigButton`
  ;[1 0.944 0 0.999] Iluminar botón
  (`MaterialInstanceDynamic.SetScalarParameterValue` (`self.DynMat`) "Intensity" 2.5)
  (`KismetSystemLibrary.Delay` 0.65)
  (`MaterialInstanceDynamic.SetScalarParameterValue` (`self.DynMat`) "Intensity" 0.0))

(event `PlayBigError`
  ; Perdiste
  (`MaterialInstanceDynamic.SetVectorParameterValue` (`self.DynMat`) "Color" (struct :`R` 1.0 :`B` 0.016275 :`A` 1.0))
  (`MaterialInstanceDynamic.SetScalarParameterValue` (`self.DynMat`) "Intensity" 5.0)
  (`KismetSystemLibrary.Delay` 0.65)
  (`MaterialInstanceDynamic.SetScalarParameterValue` (`self.DynMat`) "Intensity" 0.0)
  (`MaterialInstanceDynamic.SetVectorParameterValue` (`self.DynMat`) "Color" (`self.Color`)))

(fn `UserConstructionScript`
  (bind _returnvalue (`PrimitiveComponent.CreateDynamicMaterialInstance` (`self.TriggerButton`) 0 "/Game/EscapeRoom/Materials/M_Color.M_Color" "None"))
  (bind _output_get (set `self.DynMat` _returnvalue))
  (`MaterialInstanceDynamic.SetVectorParameterValue` _output_get "Color" (`self.Color`)))