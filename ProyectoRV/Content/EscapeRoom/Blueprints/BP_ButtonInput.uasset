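; BP_ButtonInput is a colored VR push button for a Simon-style note puzzle in the escape room.
; A VRPawn overlap on CollisionButton depresses it, plays a click, flashes it and, on the player's turn, sends its Index to SimonMainRef.
; A separate TriggerButton overlap returns it after a short delay.
; A dynamic material from the construction script drives its color, glow and victory or error feedback with sound.
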(event `self.ReceiveBeginPlay`
  ;[1 0 0.05327 0.999] Pulsar botón
  (set `self.Relative Location` (`SceneComponent.RelativeLocation` (`self.TriggerButton`))))

(event `self.CollisionButton.OnComponentBeginOverlap`
  (params (OverlappedComponent :type "PrimitiveComponent Object Reference") (OtherActor :type "Actor Object Reference") (OtherComp :type "PrimitiveComponent Object Reference") (OtherBodyIndex :type Integer) (bFromSweep :type Boolean) (SweepResult :type "HitResult Structure (by ref)"))
  ;[1 0 0.05327 0.999] Pulsar botón
  (cast `/Game/EscapeRoom/Blueprints/VRPawn` OtherActor)
  (`KismetSystemLibrary.MoveComponentTo` (`self.TriggerButton`) (- (`self.Relative Location`) (0.0 5.0 0.0)) (struct) false false 0.1)
  (`GameplayStatics.PlaySound2D` "/Game/EscapeRoom/Audio/SFX/ButtonPressed.ButtonPressed" 1.0 1.0 0.0 null null)
  (`self.LightButton`)
  (`self.TocarNota`))

(event `TocarNota`
  ; Tocar nota solo cuando sea el turno del jugador
  (bind _simonmain_ref (`self.SimonMain_Ref`)
    (:`then`
      (if (`/Game/EscapeRoom/Blueprints/BP_Simon.isPlayersTurn` _simonmain_ref)
        (`/Game/EscapeRoom/Blueprints/BP_Simon.PlayerPlayedNote` (`self.SimonMain_Ref`) (`self.Index`))))
    (:`else`)))

(event `self.TriggerButton.OnComponentBeginOverlap`
  (params (OverlappedComponent :type "PrimitiveComponent Object Reference") (OtherActor :type "Actor Object Reference") (OtherComp :type "PrimitiveComponent Object Reference") (OtherBodyIndex :type Integer) (bFromSweep :type Boolean) (SweepResult :type "HitResult Structure (by ref)"))
  ;[1 0 0.05327 0.999] Pulsar botón
  (cast `/Game/EscapeRoom/Blueprints/VRPawn` OtherActor)
  (`KismetSystemLibrary.Delay` 0.1)
  (`KismetSystemLibrary.MoveComponentTo` (`self.TriggerButton`) (`self.Relative Location`) (struct) false false 0.1))

(event `LightButton`
  ;[1 0.944 0 0.999] Iluminar botón
  (`MaterialInstanceDynamic.SetScalarParameterValue` (`self.DynMat`) "Intensity" 2.5)
  (`KismetSystemLibrary.Delay` 0.65)
  (`MaterialInstanceDynamic.SetScalarParameterValue` (`self.DynMat`) "Intensity" 0.0))

(event `PlayVictory`
  ; Ganaste
  (`GameplayStatics.PlaySound2D` "/Game/EscapeRoom/Audio/SFX/Victory.Victory" 1.0 1.0 0.0 null null)
  (`MaterialInstanceDynamic.SetVectorParameterValue` (`self.DynMat`) "Color" (struct :`G` 1.0 :`B` 0.178619 :`A` 1.0))
  (`MaterialInstanceDynamic.SetScalarParameterValue` (`self.DynMat`) "Intensity" 5.0))

(event `PlayError`
  ; Perdiste
  (`GameplayStatics.PlaySound2D` "/Game/EscapeRoom/Audio/SFX/Error.Error" 1.0 1.0 0.0 null null)
  (`MaterialInstanceDynamic.SetVectorParameterValue` (`self.DynMat`) "Color" (struct :`R` 1.0 :`B` 0.016275 :`A` 1.0))
  (`MaterialInstanceDynamic.SetScalarParameterValue` (`self.DynMat`) "Intensity" 5.0)
  (`KismetSystemLibrary.Delay` 0.65)
  (`MaterialInstanceDynamic.SetScalarParameterValue` (`self.DynMat`) "Intensity" 0.0)
  (`MaterialInstanceDynamic.SetVectorParameterValue` (`self.DynMat`) "Color" (`self.Color`)))

(fn `UserConstructionScript`
  (bind _returnvalue (`PrimitiveComponent.CreateDynamicMaterialInstance` (`self.TriggerButton`) 0 "/Game/EscapeRoom/Materials/M_Color.M_Color" "None"))
  (bind _output_get (set `self.DynMat` _returnvalue))
  (`MaterialInstanceDynamic.SetVectorParameterValue` _output_get "Color" (`self.Color`)))