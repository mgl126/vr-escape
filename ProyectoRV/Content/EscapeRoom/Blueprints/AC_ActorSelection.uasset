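; Actor component that makes its owning actor selectable when hit by the left or right hand in the escape room.
; HitActor fires once to enable owner input, apply an overlay material to the root mesh and add that hand's selection mapping context.
; IA_Selection flips Activated, calling ActorSelected when it was true and ActorDeselected otherwise.
; HitActor also retriggers a short delay, but the cleanup that would undo the hit setup is unconnected.
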(event `/Game/EscapeRoom/Blueprints/Interfaces/BPI_UserInteraction.Hit Actor`
  (params (Hand :type "EControllerHand Enum" :default "Left"))
  (bind _returnvalue (`self.GetOwner`))
  (`|ExecutionSequence`
    (:`then_0`
      (`/Engine/EditorBlueprintResources/StandardMacros.DoOnce` false
        (:`Completed`
          (`Actor.EnableInput` _returnvalue (`GameplayStatics.GetPlayerController` 0))
          (bind _asmesh_component (cast `MeshComponent` (`Actor.RootComponent` _returnvalue)))
          (bind _output_get (set `self.As Mesh Component` _asmesh_component))
          (`MeshComponent.SetOverlayMaterial` _output_get "/Game/EscapeRoom/Materials/M_Overlay.M_Overlay")
          (`EnhancedInputSubsystemInterface.AddMappingContext` (pcsubsystem `EnhancedInputLocalPlayerSubsystem` (`GameplayStatics.GetPlayerController` 0)) (select `bool` (`|EnumEquality` Hand "Right") :`false` "/Game/EscapeRoom/Input/IMC_Selection_Left.IMC_Selection_Left" :`true` "/Game/EscapeRoom/Input/IMC_Selection_Right.IMC_Selection_Right" :!type "InputMappingContext Object Reference") 0 (struct)))))
    (:`then_1`
      (`KismetSystemLibrary.RetriggerableDelay` 0.02))))

(event `EnhancedInput|/Game/EscapeRoom/Input/Action/IA_Selection`
  (params (ActionValue :type Boolean) (ElapsedSeconds :type "Float (double-precision)") (TriggeredSeconds :type "Float (double-precision)") (InputAction :type "InputAction Object Reference" :default "/Game/EscapeRoom/Input/Action/IA_Selection.IA_Selection"))
  (:`Started`
    (if (`self.Activated`)
      (set `self.Activated` false)
      (`self.Actor Selected`)
      (else
        (set `self.Activated` true)
        (`self.Actor Deselected`)))))