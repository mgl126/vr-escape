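; SC_SelectionTrace runs a selection trace from a motion controller aim in the escape room game, notifying interactable objects that a hand points at them.
; Activation stores the aim component and hand, then starts a fast looping timer that casts a short forward Visibility line trace with debug drawing.
; On a hit, it sends HitActorMessage with the hand to the actor's first BPI_UserInteraction component.
; Deactivation calls a pause on the timer by function name.
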(event `Activate Selection Trace`
  (params (MotionControllerAim :type "MotionControllerComponent Object Reference") (Hand :type "EControllerHand Enum" :default "Left"))
  (set `self.Motion Controller Aim` MotionControllerAim)
  (set `self.Hand` Hand)
  (`KismetSystemLibrary.K2_SetTimerDelegate` (delegate `Update timer`) 0.02 true))

(event `Update timer`
  (bind _motion_controller_aim (`self.Motion Controller Aim`))
  (bind _returnvalue (`self.K2_GetComponentLocation` _motion_controller_aim))
  (bind (_outhit _returnvalue_2) (`KismetSystemLibrary.LineTraceSingle` :`Start` _returnvalue :`End` (+ _returnvalue (* (`self.GetForwardVector` _motion_controller_aim) 200.0)) :`TraceChannel` "TraceTypeQuery1" :`DrawDebugType` "ForOneFrame"))
  (if _returnvalue_2
    (message `/Game/EscapeRoom/Blueprints/Interfaces/BPI_UserInteraction.Hit Actor` (`|GetArrayItem` (`Actor.GetComponentsByInterface` (`.HitActor` (`GameplayStatics.BreakHitResult` _outhit)) "/Game/EscapeRoom/Blueprints/Interfaces/BPI_UserInteraction.BPI_UserInteraction_C")) (`self.Hand`))))

(event `Deactivate Selection Trace`
  (`KismetSystemLibrary.K2_PauseTimer` null "Update timer"))