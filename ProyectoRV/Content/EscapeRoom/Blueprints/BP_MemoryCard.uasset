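; BP_MemoryCard is a card actor for a memory matching game in the escape room.
; It binds to its actor selection component's events, starting its rotating movement when selected and stopping it when deselected.
; FlipCard toggles the flipped state by snapping actor rotation between face up and face down, printing a debug message on face up, and does nothing once the card is matched.
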(event `self.ReceiveBeginPlay`
  (bind _ac_actorselection (`self.AC_ActorSelection`))
  (add `/Game/EscapeRoom/Blueprints/AC_ActorSelection.Actor Selected` _ac_actorselection (delegate `Actor Selected_Event`))
  (add `/Game/EscapeRoom/Blueprints/AC_ActorSelection.Actor Deselected` _ac_actorselection (delegate `Actor Deselected_Event`)))

(event `Actor Selected_Event`
  (`ActorComponent.Activate` (`self.RotatingMovement`) false))

(event `Actor Deselected_Event`
  (`ActorComponent.Deactivate` (`self.RotatingMovement`)))

(fn `FlipCard`
  (if (not (`self.bIsMatched`))
    (if (`self.bIsFlipped`)
      ; voltear hacia abajo
      (set `self.bIsFlipped` false)
      (`self.K2_SetActorRotation` (struct :`Pitch` 180.0))
      (return)
      (else
        ; voltear hacia arriba
        (set `self.bIsFlipped` true)
        (`self.K2_SetActorRotation` (struct))
        (`KismetSystemLibrary.PrintString` "Carta volteada")
        (return)))))

(fn `UserConstructionScript`)