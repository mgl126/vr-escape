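; BP_Simon runs a VR Simon memory puzzle, started when a VRPawn presses its physical button.
; Each level builds a random sequence from LevelSettings and plays it on paired Stands and BigStands.
; PlayerPlayedNote checks each input, advancing levels until victory or restarting from the first on a mistake.
; The construction script caps note counts at the stand count for levels without duplicates.
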(event `self.ReceiveBeginPlay`
  ;[1 0 0.05327 0.999] Mover botón con sonido
  ;; Inicializar posición botón
  (set `self.Relative Location` (`SceneComponent.RelativeLocation` (`self.TriggerButton`)))
  (`self.InitializeGame`))

(event `InitializeGame`
  ; Inicializar juego
  (for _array_element (`self.Stands`)
    (`/Engine/EditorBlueprintResources/StandardMacros.IsValid` _array_element
      (:`Is Valid`
        (set `/Game/EscapeRoom/Blueprints/BP_ButtonInput.SimonMain_Ref` self _array_element))
      (:`Is Not Valid`
        (`KismetSystemLibrary.PrintString` "Error al inicializar los botones" true true (struct :`R` 1.0 :`G` 0.868307 :`A` 1.0) 5.0)))))

(event `self.CollisionButton.OnComponentBeginOverlap`
  (params (OverlappedComponent :type "PrimitiveComponent Object Reference") (OtherActor :type "Actor Object Reference") (OtherComp :type "PrimitiveComponent Object Reference") (OtherBodyIndex :type Integer) (bFromSweep :type Boolean) (SweepResult :type "HitResult Structure (by ref)"))
  ;[1 0 0.05327 0.999] Mover botón con sonido
  ;; Mover botón hacia abajo
  (cast `/Game/EscapeRoom/Blueprints/VRPawn` OtherActor)
  (`KismetSystemLibrary.MoveComponentTo` (`self.TriggerButton`) (- (`self.Relative Location`) (0.0 0.0 2.0)) (struct) false false 0.1)
  (`GameplayStatics.PlaySound2D` "/Game/EscapeRoom/Audio/SFX/ButtonPressed.ButtonPressed" 1.0 1.0 0.0 null null)
  (`self.StartGame`))

(event `AddAnotherNote`
  (bind (_numberofnotes _timebetweennotes _canduplicatenotes) (break `/Game/EscapeRoom/Blueprints/Simon_LevelStructure` (`|GetArrayItem` (`self.LevelSettings`) (`self.CurrentLevel`))))
  ; Crear secuencia aleatoria basada en el nivel
  (if (> (`KismetArrayLibrary.Array_Length` (`self.Stands`)) 0) :!label _label
    (if _canduplicatenotes
      (`KismetArrayLibrary.Array_Add` (`self.SimonSequence`) (`KismetMathLibrary.RandomIntegerInRange` 0 (`KismetArrayLibrary.Array_LastIndex` (`self.Stands`))))
      (else
        (`KismetArrayLibrary.Array_AddUnique` (`self.SimonSequence`) (`KismetMathLibrary.RandomIntegerInRange` 0 (`KismetArrayLibrary.Array_LastIndex` (`self.Stands`))))))
    (if (< (`KismetArrayLibrary.Array_Length` (`self.SimonSequence`)) _numberofnotes)
      (`KismetSystemLibrary.Delay` 0.0)
      (`self.AddAnotherNote`)
      (else
        (`KismetSystemLibrary.Delay` 1.0)
        (`self.PlaySimonSequence`)))))

(event `CreateSimonSequence`
  ; Crear secuencia aleatoria basada en el nivel
  (`KismetArrayLibrary.Array_Clear` (`self.SimonSequence`))
  (goto _label))

(event `StartGame`
  ; Overlap Event
  (if (not (`self.isPlaying`))
    (set `self.isPlaying` true)
    (`self.StartLevel`)))

(event `self.TriggerButton.OnComponentBeginOverlap`
  (params (OverlappedComponent :type "PrimitiveComponent Object Reference") (OtherActor :type "Actor Object Reference") (OtherComp :type "PrimitiveComponent Object Reference") (OtherBodyIndex :type Integer) (bFromSweep :type Boolean) (SweepResult :type "HitResult Structure (by ref)"))
  ;[1 0 0.05327 0.999] Mover botón con sonido
  ;; Mover botón hacia arriba
  (cast `/Game/EscapeRoom/Blueprints/VRPawn` OtherActor)
  (`KismetSystemLibrary.Delay` 0.1)
  (`KismetSystemLibrary.MoveComponentTo` (`self.TriggerButton`) (`self.Relative Location`) (struct) false false 0.1))

(event `StartLevel`
  ; Empezar nivel
  (`KismetArrayLibrary.Array_Clear` (`self.PlayerSequence`))
  (set `self.CurrentNote` 0)
  (set `self.isPlayersTurn` false)
  (`self.CreateSimonSequence`))

(event `PlaySimonSequence`
  ; Reproducir secuencia creada
  (`/Game/EscapeRoom/Blueprints/BP_ButtonInput.LightButton` (`|GetArrayItem` (`self.Stands`) (`|GetArrayItem` (`self.SimonSequence`) (`self.CurrentNote`))))
  (`/Game/EscapeRoom/Blueprints/BP_BigButton.LightBigButton` (`|GetArrayItem` (`self.BigStands`) (`|GetArrayItem` (`self.SimonSequence`) (`self.CurrentNote`))))
  (`KismetSystemLibrary.Delay` (`.TimeBetweenNotes_4_ABD540374A724347A030A387D222EEE8` (break `/Game/EscapeRoom/Blueprints/Simon_LevelStructure` (`|GetArrayItem` (`self.LevelSettings`) (`self.CurrentLevel`)))))
  (`/Engine/EditorBlueprintResources/StandardMacros.IncrementInt` (`self.CurrentNote`)
    (:`  `
      (if (< (`self.CurrentNote`) (`KismetArrayLibrary.Array_Length` (`self.SimonSequence`)))
        (`self.PlaySimonSequence`)
        (else
          (set `self.isPlayersTurn` true))))))

(event `PlayerPlayedNote`
  (params (Note :type Integer))
  ; Jugador toca un botón
  (set `self.isPlayersTurn` false)
  (bind _returnvalue (`KismetArrayLibrary.Array_Add` (`self.PlayerSequence`) Note))
  (if (== Note (`|GetArrayItem` (`self.SimonSequence`) _returnvalue))
    (`/Game/EscapeRoom/Blueprints/BP_ButtonInput.LightButton` (`|GetArrayItem` (`self.Stands`) Note))
    (if (>= (`KismetArrayLibrary.Array_Length` (`self.PlayerSequence`)) (`KismetArrayLibrary.Array_Length` (`self.SimonSequence`)))
      (if (< (`self.CurrentLevel`) (`KismetArrayLibrary.Array_LastIndex` (`self.LevelSettings`)))
        (`/Engine/EditorBlueprintResources/StandardMacros.IncrementInt` (`self.CurrentLevel`)
          (:`  `
            (`KismetSystemLibrary.Delay` 2.0)
            (`self.StartLevel`)))
        (else
          ; Ganaste
          (for _array_element (`self.Stands`)
            (`/Game/EscapeRoom/Blueprints/BP_ButtonInput.PlayVictory` _array_element)
            (for _array_element_2 (`self.BigStands`)
              (`/Game/EscapeRoom/Blueprints/BP_BigButton.PlayBigVictory` _array_element_2)))))
      (else
        (set `self.isPlayersTurn` true)))
    (else
      ; Perdiste
      (for _array_element_3 (`self.Stands`)
        (`/Game/EscapeRoom/Blueprints/BP_ButtonInput.PlayError` _array_element_3)
        (for _array_element_4 (`self.BigStands`)
          (`/Game/EscapeRoom/Blueprints/BP_BigButton.PlayBigError` _array_element_4)))
      (`KismetSystemLibrary.Delay` 2.0)
      (set `self.CurrentLevel` 0)
      (`self.StartLevel`))))

(fn `UserConstructionScript`
  (bind _returnvalue (`KismetArrayLibrary.Array_Length` (`self.Stands`)))
  (for (_array_element _array_index) (`self.LevelSettings`)
    (bind (_numberofnotes _timebetweennotes _canduplicatenotes) (break `/Game/EscapeRoom/Blueprints/Simon_LevelStructure` _array_element))
    (if _canduplicatenotes
      _
      (elif (> _numberofnotes _returnvalue)
        (bind _structout (setmembers `/Game/EscapeRoom/Blueprints/Simon_LevelStructure` :`StructRef` _array_element :`NumberOfNotes` _returnvalue))
        (`KismetArrayLibrary.Array_Set` (`self.LevelSettings`) _array_index _structout)))))